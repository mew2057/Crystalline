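; Blinking point light Blueprint, named as a red light, that switches itself on and off about once a second.
; Tick accumulates delta time in TimeElap, then resets it and flips the On boolean each time it reaches one second.
; The On state drives the PointLightComponent intensity between full brightness and zero, with no timer or timeline involved.
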(event EventBeginPlay)

(event EventTick
  (params (DeltaSeconds :type Float%20%28single-precision%29))
  (bind _pointlightcomponent (Variables|Default|GetPointLightComponent))
  (Variables|Default|SettimeElap (+ DeltaSeconds (Variables|Default|GettimeElap)))
  (if (>= (Variables|Default|GettimeElap) 1.0)
    (Variables|Default|SettimeElap 0.0)
    (if (Variables|Default|Geton)
      (Variables|Default|Seton false)
      (else
        (Variables|Default|Seton true)))
    (if (Variables|Default|Geton)
      (Rendering|Components|Light|SetIntensity _pointlightcomponent 5e+03)
      (else
        (Rendering|Components|Light|SetIntensity _pointlightcomponent 0.0)))))

(fn ConstructionScript)