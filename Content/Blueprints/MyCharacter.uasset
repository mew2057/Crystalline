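; MyCharacter is a character Blueprint that fires projectiles when the left mouse button is pressed.
; The press calls the ServerAttemptSpawnBullet event, which runs SpawnBullet.
; SpawnBullet acts only with authority, spawning a Projectile at a gun offset rotated by control rotation, even if colliding.
; The weapon fire sound plays at the actor's location in that same authority-only branch.
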(event Custom|ServerAttemptSpawnBullet
  (CallFunction|SpawnBullet))

(event Input|MouseEvents|LeftMouseButton
  (:Pressed
    (CallFunction|ServerAttemptSpawnBullet)))

(fn ConstructionScript)

(fn SpawnBullet
  (bind _returnvalue (Pawn|GetControlRotation :!class /Script/Engine.Pawn))
  (Networking|SwitchHasAuthority
    (:Authority
      (Game|SpawnActorfromClass "/Game/Blueprints/Projectile.Projectile_C" (Math|Transform|MakeTransform (+ (Transformation|GetActorLocation) (Math|Vector|RotateVector (Variables|Default|GetGunOffset) _returnvalue)) _returnvalue) true 0)
      (Audio|PlaySoundatLocation "/Game/Audio/Template1rst_WeaponFire02.Template1rst_WeaponFire02" (Transformation|GetActorLocation)))))