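; Menu HUD that draws the main menu (Host, Join, Quit, IP field) and lobby (Quit, server-only Start) for a networked game.
; DrawHUD paints a back-and-forth parallax background, then texture buttons with centered text, each registering a hit box named after its label.
; Key events edit the IP string.
; Hit-box clicks set pressed textures, and releases run console commands to host, join, exit or server-travel to the game level.
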(event EventDrawHUD
  (params (SizeX :type Integer) (SizeY :type Integer))
  (bind _returnvalue (Math|Float|MakeLiteralFloat 4e+02))
  (bind _returnvalue_2 (Math|Float|MakeLiteralFloat 3.5e+02))
  (bind _buttontexture (Variables|Default|GetButtonTexture))
  ;[1 1 1] Get Sizes of Screen
  (Variables|Default|SetButtonSize (Math|Vector2D|MakeVector2D (Math|Conversions|ToFloat(Integer) (Class|Texture2D|BlueprintGetSizeX _buttontexture)) (Math|Conversions|ToFloat(Integer) (Class|Texture2D|BlueprintGetSizeY _buttontexture))))
  (Variables|Default|SetScreenDimensions (Math|Vector2D|MakeVector2D (Math|Conversions|ToFloat(Integer) SizeX) (Math|Conversions|ToFloat(Integer) SizeY)))
  (CallFunction|DrawBackground (Variables|Default|GetDeltaTime))
  ;[1 1 1] Draw Menu Screen
  (if (Variables|Default|GetMainMenuIsActive)
    ;;[1 1 1] Draw IP String
    (HUD|DrawRect (Variables|Default|GetTextBackgroundColor) _returnvalue _returnvalue_2 (Math|Float|MakeLiteralFloat 4e+02) (Math|Float|MakeLiteralFloat 5e+01))
    (HUD|DrawText (Variables|Default|GetipString) (Variables|Default|GetTextColor) _returnvalue _returnvalue_2 "/Game/Textures/HUD/MenuFont.MenuFont" 1.0 false)
    (CallFunction|DrawMenuButton 1e+01 2e+02 (Variables|Default|GetHostButtonPressed) "Host")
    (CallFunction|DrawMenuButton 1e+01 3e+02 (Variables|Default|GetJoinButtonPressed) "Join")
    (CallFunction|DrawMenuButton 1e+01 4e+02 (Variables|Default|GetQuitButtonPressed) "Quit")
    (else
      ;[1 1 1] Draw Lobby Screen
      (if (Variables|Default|GetLobbyIsActive)
        (if (Networking|IsServer)
          (CallFunction|DrawMenuButton 1e+01 3e+02 (Variables|Default|GetStartButtonPressed) "Start"))
        (CallFunction|DrawMenuButton 1e+01 4e+02 (Variables|Default|GetQuitButtonPressed) "Quit")))))

(event EventHitBoxClick
  (params (BoxName :type Name :default "None"))
  ;[1 1 1] On button clicks
  (switch name BoxName
    (:Host
      (Variables|Default|SetHostButtonPressed true))
    (:Join
      (Variables|Default|SetJoinButtonPressed true))
    (:Quit
      (Variables|Default|SetQuitButtonPressed true))
    (:Start
      (Variables|Default|SetStartButtonPressed true))))

(event EventHitBoxRelease
  (params (BoxName :type Name :default "None"))
  (bind _returnvalue (Utilities|String|MakeLiteralString "Travel "))
  (switch name BoxName
    (:Host
      (Development|ExecuteConsoleCommand (Utilities|String|Append _returnvalue (Utilities|String|MakeLiteralString "LobbyLevel?Listen"))))
    (:Join
      (Development|ExecuteConsoleCommand (Utilities|String|Append _returnvalue (Variables|Default|GetipString))))
    (:Quit
      (Development|ExecuteConsoleCommand "Exit"))
    (:Start
      (Variables|Default|SetLobbyIsActive false)
      (Variables|Default|SetMainMenuIsActive false)
      (Development|ExecuteConsoleCommand (Utilities|String|Append (Utilities|String|MakeLiteralString "ServerTravel ") (Variables|Default|GetGameLevelName))))))

(event EventTick
  (params (DeltaSeconds :type Float%20%28single-precision%29))
  (Variables|Default|SetDeltaTime DeltaSeconds))

(event Input|KeyboardEvents|1
  ;[1 1 1] Get Input
  (:Pressed
    (CallFunction|BuildHostString "1")))

(event Input|KeyboardEvents|2
  ;[1 1 1] Get Input
  (:Pressed
    (CallFunction|BuildHostString "2")))

(event Input|KeyboardEvents|3
  ;[1 1 1] Get Input
  (:Pressed
    (CallFunction|BuildHostString "3")))

(event Input|KeyboardEvents|4
  ;[1 1 1] Get Input
  (:Pressed
    (CallFunction|BuildHostString "4")))

(event Input|KeyboardEvents|5
  ;[1 1 1] Get Input
  (:Pressed
    (CallFunction|BuildHostString "5")))

(event Input|KeyboardEvents|7
  ;[1 1 1] Get Input
  (:Pressed
    (CallFunction|BuildHostString "7")))

(event Input|KeyboardEvents|6
  ;[1 1 1] Get Input
  (:Pressed
    (CallFunction|BuildHostString "6")))

(event Input|KeyboardEvents|8
  ;[1 1 1] Get Input
  (:Pressed
    (CallFunction|BuildHostString "8")))

(event Input|KeyboardEvents|9
  ;[1 1 1] Get Input
  (:Pressed
    (CallFunction|BuildHostString "9")))

(event Input|KeyboardEvents|0
  ;[1 1 1] Get Input
  (:Pressed
    (CallFunction|BuildHostString "0")))

(event Input|KeyboardEvents|Period
  ;[1 1 1] Get Input
  (:Pressed
    (CallFunction|BuildHostString ".")))

(event Input|KeyboardEvents|Backspace
  ;[1 1 1] Get Input
  (:Pressed
    (CallFunction|DeleteStringCharacter)))

(event Input|KeyboardEvents|Delete
  ;[1 1 1] Get Input
  (:Pressed
    (CallFunction|DeleteStringCharacter)))

(event Input|MouseEvents|LeftMouseButton
  (:Released
    (Variables|Default|SetHostButtonPressed false)
    (Variables|Default|SetJoinButtonPressed false)
    (Variables|Default|SetQuitButtonPressed false)
    (Variables|Default|SetStartButtonPressed false)))

(fn ConstructionScript)

(fn DrawButton
  (params (ButtonScreenLocation :type Vector%202D%20Structure) (BUttonSize :type Vector%202D%20Structure) (ButtonText :type String) (Texture :type Texture%20Object%20Reference) (TextColor :type Linear%20Color%20Structure))
  (bind (_x _y) (Math|Vector2D|BreakVector2D ButtonScreenLocation))
  (bind (_outwidth _outheight) (Class|HUD|GetTextSize ButtonText "/Game/Textures/HUD/MenuFont.MenuFont" 1.0))
  (bind _returnvalue (/ BUttonSize 2.0))
  (bind _returnvalue_2 (Math|Vector2D|MakeVector2D _outwidth _outheight))
  (bind _returnvalue_3 (+ ButtonScreenLocation _returnvalue))
  (bind _returnvalue_4 (/ _returnvalue_2 2.0))
  (bind _returnvalue_5 (- _returnvalue_3 _returnvalue_4))
  (bind (_x_2 _y_2) (Math|Vector2D|BreakVector2D _returnvalue_5))
  (Class|HUD|DrawTextureSimple Texture _x _y 1.0 false)
  (HUD|DrawText ButtonText TextColor _x_2 _y_2 "/Game/Textures/HUD/MenuFont.MenuFont" 1.0 false)
  (Class|HUD|AddHitBox ButtonScreenLocation BUttonSize (Utilities|String|StringToName ButtonText) false))

(fn BuildHostString
  (params (KeyInput :type String))
  (Variables|Default|SetipString (Utilities|String|Append (Variables|Default|GetipString) KeyInput)))

(fn DeleteStringCharacter
  (Variables|Default|SetipString (Utilities|String|GetSubstring (Variables|Default|GetipString) 0 (- (Utilities|String|Len (Variables|Default|GetipString)) 1))))

(fn DrawMenuButton
  (params (LocationX :type Float%20%28single-precision%29) (LocationY :type Float%20%28single-precision%29) (IsPressed :type Boolean) (ButtonText :type String))
  (CallFunction|DrawButton (Math|Vector2D|MakeVector2D LocationX LocationY) (Variables|Default|GetButtonSize) ButtonText (select IsPressed (Variables|Default|GetBUttonTexturePressed) (Variables|Default|GetButtonTexture)) (Variables|Default|GetTextColor)))

(fn DrawBackground
  (params (DeltaTime :type Float%20%28single-precision%29))
  (Variables|Default|SetBackgroundShift (+ (* DeltaTime 0.05) (Variables|Default|GetBackgroundShift)))
  (if (> (Math|Float|%(Float) (Variables|Default|GetBackgroundShift) 2.0) 1.0)
    (Variables|Default|SetChangedShift (Math|Float|%(Float) (Variables|Default|GetBackgroundShift) 2.0))
    (else
      (Variables|Default|SetChangedShift (- 2.0 (Math|Float|%(Float) (Variables|Default|GetBackgroundShift) 2.0)))))
  (Class|HUD|DrawTextureSimple "/Game/Textures/menuBack.menuBack" (- 1.2e+02 (* (Variables|Default|GetChangedShift) 1.2e+02)) 0.0 0.8 false)
  (Class|HUD|DrawTextureSimple "/Game/Textures/menuMid.menuMid" 0.0 0.0 0.8 false)
  (Class|HUD|DrawTextureSimple "/Game/Textures/menuFront.menuFront" (* (- 2.0 (Variables|Default|GetChangedShift)) -1.8e+02) 0.0 0.8 false))