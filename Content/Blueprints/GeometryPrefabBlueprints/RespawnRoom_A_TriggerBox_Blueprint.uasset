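; Respawn room trigger box that repositions its Door actor when an overlap with the box ends.
; The end-overlap event switches on DoorNum and snaps Door to a hard-coded relative location for that door, with no sweep or interpolation.
; Only certain door numbers are handled, and the overlapping actor is not filtered.
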(event OnComponentEndOverlap(TriggerBox_0)
  (params (OtherActor :type Actor%20Object%20Reference) (OtherComp :type Primitive%20Component%20Object%20Reference) (OtherBodyIndex :type Integer))
  (bind _door (Variables|Default|GetDoor))
  (switch int (Variables|Default|GetdoorNum)
    (:1
      (Transformation|SetActorRelativeLocation _door "4536.000000,3056.000000,288.000000"))
    (:3
      (Transformation|SetActorRelativeLocation _door "6840.000000,200.000000,544.000000"))
    (:5
      (Transformation|SetActorRelativeLocation _door "4536.000000,-2616.000000,288.000000"))
    (:7
      (Transformation|SetActorRelativeLocation _door "-4536.000000,3024.000000,288.000000"))
    (:9
      (Transformation|SetActorRelativeLocation _door "-4536.000000,-2616.000000,288.000000"))
    (:11
      (Transformation|SetActorRelativeLocation _door "-6840.000000,200.000000,544.000000"))
    (:13
      (Transformation|SetActorRelativeLocation _door "-1903.156738,-4714.766113,536.000000"))
    (:15
      (Transformation|SetActorRelativeLocation _door "1542.863281,4864.677734,544.000000"))
    (:18
      (Transformation|SetActorRelativeLocation _door "2002.966553,-4674.548828,544.000000"))
    (:20
      (Transformation|SetActorRelativeLocation _door "-1990.151367,4675.869141,544.000000"))))

(fn ConstructionScript)