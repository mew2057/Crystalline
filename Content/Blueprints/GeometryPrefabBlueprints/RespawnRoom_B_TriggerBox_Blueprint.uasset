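; Respawn room trigger box that acts when an actor's overlap with it ends.
; A departing CGPlayer has all crystals popped from its inventory.
; For any departing actor, player or not, DoorNum selects a hard-coded relative location to which the referenced Door snaps without sweep.
; Case 12 is the exception, moving the Blueprint's own actor instead of Door.
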(event OnComponentEndOverlap(TriggerBox_0)
  (params (OtherActor :type Actor%20Object%20Reference) (OtherComp :type Primitive%20Component%20Object%20Reference) (OtherBodyIndex :type Integer))
  (bind _door (Variables|Default|GetDoor))
  (Utilities|FlowControl|Sequence
    (:then_0
      (bind _ascgplayer (Utilities|Casting|CastToCGPlayer OtherActor))
      (Class|CGInventory|PopAllCrystals (Variables|/Script/Crystalline.CGCharacter|GetInventory _ascgplayer)))
    (:then_1
      (switch int (Variables|Default|GetDoorNum)
        (:2
          (Transformation|SetActorRelativeLocation _door "3576.000000,3056.000000,288.000000"))
        (:4
          (Transformation|SetActorRelativeLocation _door "5880.000000,200.000000,544.000000"))
        (:6
          (Transformation|SetActorRelativeLocation _door "3576.000000,-2616.000000,288.000000"))
        (:8
          (Transformation|SetActorRelativeLocation _door "-3576.000000,3024.000000,288.000000"))
        (:10
          (Transformation|SetActorRelativeLocation _door "-3576.000000,-2616.000000,288.000000"))
        (:12
          (Transformation|SetActorRelativeLocation "-5880.000000,200.000000,544.000000"))
        (:14
          (Transformation|SetActorRelativeLocation _door "-1530.112305,-3830.208984,544.000000"))
        (:16
          (Transformation|SetActorRelativeLocation _door "1178.222900,3976.586182,544.000000"))
        (:17
          (Transformation|SetActorRelativeLocation _door "1623.577148,-3792.663086,544.000000"))
        (:19
          (Transformation|SetActorRelativeLocation _door "-1605.636719,3796.202148,544.000000"))))))

(fn ConstructionScript)