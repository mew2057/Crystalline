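; BP_CapturePoint is a King of the Hill capture zone meant to award score to players inside it.
; Overlap events add and remove CGPlayers in PlayersInZone, while Tick accumulates time and, each second, calls UpdateScore on KotH_GameMode with a player state.
; That player state derives from a loop element over PlayersInZone, but the loop is not wired into execution, so it never iterates.
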(event EventBeginPlay)

(event EventActorBeginOverlap
  (params (OtherActor :type Actor%20Object%20Reference))
  (bind _ascgplayer (Utilities|Casting|CastToCGPlayer OtherActor))
  (Utilities|Array|Add (Variables|Default|GetplayersInZone) _ascgplayer))

(event EventTick
  (params (DeltaSeconds :type Float%20%28single-precision%29))
  (Variables|Default|SettimeElap (+ DeltaSeconds (Variables|Default|GettimeElap)))
  (if (>= (Variables|Default|GettimeElap) 1.0)
    (Variables|Default|SettimeElap 0.0)
    (bind _askot_h_game_mode (Utilities|Casting|CastToKotH_GameMode (Game|GetGameMode)))
    (bind _ascgplayer_state (Utilities|Casting|CastToCGPlayerState (Variables|/Script/Engine.Controller|GetPlayerState (Pawn|GetController (Variables|/Script/Engine.Actor|GetInstigator (stale _array_element))))))
    (Default|UpdateScore _askot_h_game_mode _ascgplayer_state)))

(event EventActorEndOverlap
  (params (OtherActor :type Actor%20Object%20Reference))
  (bind _ascgplayer (Utilities|Casting|CastToCGPlayer OtherActor))
  (Utilities|Array|RemoveItem (Variables|Default|GetplayersInZone) _ascgplayer))

(fn ConstructionScript)